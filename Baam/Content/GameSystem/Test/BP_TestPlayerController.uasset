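; BP_TestPlayerController is a test player controller for a Bang-style card game.
; On BeginPlay the local controller creates the WBP_BangHUD widget, adds it to the viewport and shows the mouse cursor.
; Debug keys drive game logic: one asks BP_TestGamemode to assign roles, another requests playing a Beer card by gameplay tag on a target seat.
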(event EventBeginPlay
  (if (Pawn|IsLocalPlayerController)
    (bind _returnvalue (UserInterface|CreateWidget "/Game/UI/WBP_BangHUD.WBP_BangHUD_C"))
    (UserInterface|Viewport|AddtoViewport _returnvalue 0)
    (Variables|Default|SetbShowMouseCursor true)))

(event EventTick
  (params (DeltaSeconds :type Float%20%28single-precision%29)))

(event Input|KeyboardEvents|3
  (params (Key :type Key%20Structure :default "None"))
  (:Pressed
    (bind _asbp_test_gamemode (Utilities|Casting|CastToBP_TestGamemode (Game|GetGameMode)))
    (Class|BaamGameMode|AssignRoles _asbp_test_gamemode)))

(event Input|KeyboardEvents|4
  (params (Key :type Key%20Structure :default "None"))
  (:Pressed
    (Class|BaamPlayerController|RequestPlayCardbyTag "(TagName=\"Card.Id.Beer\")")))

(fn ConstructionScript)